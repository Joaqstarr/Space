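; Gameplay ability for the player ship's sword swing, with motion warping toward a target.
; On commit, an instant capsule target actor gathers candidates from the owner's transform, and a failed commit cancels the ability.
; Valid data sets the "SwordTarget" warp to a random gathered actor, or to none if empty.
; The swing montage plays even if targeting is cancelled, and its completion or interruption ends the ability.
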(event Ability|EventActivateAbility
  (bind _returnvalue (Ability|GetActorInfo))
  (bind _returnvalue_2 (Ability|CommitAbility))
  (if _returnvalue_2
    (bind _data (|WaitTargetData :ConfirmationType "Instant" :Class "/Game/Space/Actors/GameplayAbilityTargetingActors/BP_CapsuleTarget.BP_CapsuleTarget_C" :StartLocation (Utilities|Struct|MakeGameplayAbilityTargetingLocationInfo "ActorTransform" (Transformation|GetActorTransform (.owneractor _returnvalue)) (.owneractor _returnvalue)) :ReticleClass 0)
      (:ValidData
        (CallFunction|SetMotionWarp _data))
      (:Cancelled
        _))
    (Animation|Montage|PlayMontage (.skeletalmeshcomponent (Ability|GetActorInfo)) "/Game/Space/Player/Art/Montages/AM_SwordSwing.AM_SwordSwing"
      (:OnCompleted
        _)
      (:OnInterrupted
        _))
    (Ability|EndAbility)
    (else
      (Ability|CancelAbility))))

(event Ability|EventOnEndAbility
  (params (bWasCancelled :type Boolean)))

(fn SetMotionWarp
  (params (TargetData :type Gameplay%20Ability%20Target%20Data%20Handle%20Structure%20%28by%20ref%29))
  (bind _returnvalue (Ability|TargetData|GetAllActorsfromTargetData TargetData))
  (bind _asplayer_ship (Utilities|Casting|CastToPlayerShip (.AvatarActor (Utilities|Struct|BreakGameplayAbilityActorInfo (Ability|GetActorInfo)))))
  (if (> (Utilities|Array|Length _returnvalue) 0)
    (Class|SwordSwingAbility|AddMotionWarpingTarget "SwordTarget" (.OutItem (Utilities|Array|Random _returnvalue)) _asplayer_ship)
    (else
      (Class|SwordSwingAbility|AddMotionWarpingTarget "SwordTarget" 0 _asplayer_ship)))
  (return))