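; BP_Sword is a player weapon Blueprint that animates a sword growing and shrinking as it is enabled and disabled.
; EnableSword and DisableSword extend their parent events, playing separate timelines that drive the mesh's Y world scale while X and Z stay fixed.
; BeginPlay calls DisableSword, so the shrink animation runs at spawn and the sword begins in its disabled state.
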(event EventBeginPlay
  (Class|Sword|DisableSword))

(event Collision|EventActorBeginOverlap
  (params (OtherActor :type Actor%20Object%20Reference)))

(event EventTick
  (params (DeltaSeconds :type Float%20%28single-precision%29)))

(event EventEnableSword
  (|CallParentFunction)
  (bind _swordscale (Timeline|GrowSword PlayFromStart)
    (:Update
      (Transformation|SetWorldScale3D (Variables|Default|GetSwordMesh) (Math|Vector|MakeVector 1e+02 _swordscale 1e+02)))))

(event EventDisableSword
  (|CallParentFunction)
  (bind _swordscale (Timeline|ShrinkTimeline PlayFromStart)
    (:Update
      (Transformation|SetWorldScale3D (Variables|Default|GetSwordMesh) (Math|Vector|MakeVector 1e+02 _swordscale 1e+02)))))

(fn ConstructionScript)