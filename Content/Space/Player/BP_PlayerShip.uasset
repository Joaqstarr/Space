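; Player-controlled spaceship pawn that turns Enhanced Input into flight controls and shows the ship HUD.
; On possession it creates and initializes WB_ShipUi with itself, and on BeginPlay it adds its input mapping context.
; Mouse deltas update a stored mouse position that Tick feeds into yaw and pitch like a virtual stick, alongside polled roll and three-axis thrust input.
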(event Input|EnhancedActionEvents|EnhancedInputActionIA_PitchYaw
  (params (ActionValue :type Vector%202D%20Structure) (ElapsedSeconds :type Float%20%28double-precision%29) (TriggeredSeconds :type Float%20%28double-precision%29) (InputAction :type Input%20Action%20Object%20Reference :default "/Game/Space/Input/IA_PitchYaw.IA_PitchYaw"))
  (Class|PlayerShip|UpdateMousePos (Math|Vector2D|MakeVector2D (.x ActionValue) (.y ActionValue))))

(event EventBeginPlay
  (Utilities|AddInputMappingContext (Variables|Default|GetInputMappingContext)))

(event Collision|EventActorBeginOverlap
  (params (OtherActor :type Actor%20Object%20Reference)))

(event EventTick
  (params (DeltaSeconds :type Float%20%28single-precision%29))
  (bind _returnvalue (Class|PlayerShip|GetMousePos true))
  (bind _returnvalue_2 (Input|EnhancedActionValues|GetIA_Move))
  (Class|Ship|AddYaw (.x _returnvalue))
  (Class|Ship|AddPitch (.y _returnvalue))
  (Class|Ship|AddRoll (Input|EnhancedActionValues|GetIA_Roll))
  (Class|Ship|AddThrust (.y _returnvalue_2) (.x _returnvalue_2) (.z _returnvalue_2)))

(event EventPossessed
  (params (NewController :type Controller%20Object%20Reference))
  (bind _asplayer_controller (Utilities|Casting|CastToPlayerController NewController))
  (bind _returnvalue (UserInterface|CreateWidget "/Game/Space/UI/WB_ShipUi.WB_ShipUi_C" _asplayer_controller))
  (Default|Initialize _returnvalue self)
  (UserInterface|Viewport|AddtoViewport _returnvalue 0))

(fn ConstructionScript)