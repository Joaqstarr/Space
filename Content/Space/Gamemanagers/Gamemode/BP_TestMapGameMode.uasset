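; Test map game mode that exercises the token allocation of the enemy manager world subsystem.
; On BeginPlay it sets a token pool and registers three consumers with different priorities.
; It then prints the tokens assigned to each consumer as a debug string.
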(event EventBeginPlay
  (bind _returnvalue (Subsystems|GetEnemyManagerWorldSubsystem))
  (bind _returnvalue_2 (Subsystems|GetEnemyManagerWorldSubsystem))
  (Class|EnemyManagerWorldSubsystem|SetTokens _returnvalue_2 100)
  (Class|EnemyManagerWorldSubsystem|RegisterTokenConsumer _returnvalue_2 0 5)
  (Class|EnemyManagerWorldSubsystem|RegisterTokenConsumer _returnvalue_2 1 90)
  (Class|EnemyManagerWorldSubsystem|RegisterTokenConsumer _returnvalue_2 2 45)
  (Development|PrintString (Utilities|String|Append (Utilities|String|ToString(Integer) (Class|EnemyManagerWorldSubsystem|GetAssignedTokens _returnvalue)) "|" (Utilities|String|ToString(Integer) (Class|EnemyManagerWorldSubsystem|GetAssignedTokens _returnvalue 1)) "|" (Utilities|String|ToString(Integer) (Class|EnemyManagerWorldSubsystem|GetAssignedTokens _returnvalue 2)))))

(fn ConstructionScript)