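; Enemy turret actor that tracks an assigned target and fires pooled projectiles at it.
; Each tick it feeds the target's position and velocity, plus the projectile class's max speed, to LookAt for aiming, then fires Gun.
; With no valid target, it aims along the gun's forward vector without firing.
; Construction links BulletPool to Gun and caches its projectile class; SetTarget supplies the target externally.
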(event EventBeginPlay)

(event EventTick
  (params (DeltaSeconds :type Float%20%28single-precision%29))
  (bind _lookat (Variables|Default|GetLookAt))
  (bind _targetactor (Variables|Default|GetTargetActor))
  (bind _gun (Variables|Default|GetGun))
  (if (Utilities|IsValid _targetactor)
    (Class|LookatComponent|UpdateLookPosition _lookat (.location (Transformation|GetActorTransform _targetactor)) (Transformation|GetVelocity _targetactor) (.MaxSpeed (Utilities|GetClassDefaults (Variables|Default|GetProjectileToPool))))
    (Class|GunComponent|Fire (Variables|Default|GetGun))
    (else
      (Class|LookatComponent|UpdateLookPosition _lookat (+ (Math|Vector|GetForwardVector _gun) (Transformation|GetWorldLocation _gun)) (Math|Vector|VectorZero) 1.0))))

(fn ConstructionScript
  (Variables|/Script/Space.GunComponent|SetProjectilePool (Variables|Default|GetGun) (Variables|Default|GetBulletPool))
  (bind _returnvalue (Class|PoolManagerComponent|GetClasstoPool (Variables|Default|GetBulletPool)))
  (bind _asprojectile (Utilities|Casting|CastToProjectileClass _returnvalue)
    (:then
      (Variables|Default|SetProjectileToPool _asprojectile))
    (:CastFailed
      (Variables|Default|SetProjectileToPool _asprojectile)
      (Development|PrintString "Projectile pool is not a projectile"))))

(fn SetTarget
  (params (NewTarget :type Actor%20Object%20Reference))
  (Variables|Default|SetTargetActor NewTarget))