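; BP_TurretController is the AI controller for enemy turrets, handing the player's ship to the turret as its target.
; On possession it caches the pawn as a BP_Turret.
; Its Vision perception component sets the target when a BP_PlayerShip is sensed and clears it when sensing is lost.
; The general perception-updated handler loops over updated actors but does nothing.
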(event OnTargetPerceptionUpdated(Vision)
  (params (Actor :type Actor%20Object%20Reference) (Stimulus :type AI%20Stimulus%20Structure))
  (if (Class|GameplayStatics|ObjectIsA Actor "/Game/Space/Player/BP_PlayerShip.BP_PlayerShip_C")
    (bind _asturret (Variables|Default|GetAsTurret)
      (:then
        (if (.bSuccessfullySensed (Utilities|Struct|BreakAIStimulus Stimulus))
          (Default|SetTarget _asturret Actor)
          (else
            (Default|SetTarget _asturret))))
      (:else))))

(event OnPerceptionUpdated(Vision)
  (params (UpdatedActors :type Array%20of%20Actor%20Object%20References))
  (for _array_element UpdatedActors
    _))

(event EventPossess
  (params (PossessedPawn :type Pawn%20Object%20Reference))
  (bind _asbp_turret (Utilities|Casting|CastToBP_Turret PossessedPawn))
  (Variables|Default|SetAsTurret _asbp_turret))

(fn ConstructionScript)