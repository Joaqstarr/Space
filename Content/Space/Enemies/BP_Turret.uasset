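; Enemy turret for the space game that tracks the player ship and fires at it continuously.
; Finds BP_PlayerShip on BeginPlay, then each tick feeds its position, velocity and the projectile's max speed to LookAt for lead aiming, and calls Gun.Fire.
; The construction script assigns BulletPool to the Gun and caches the pooled projectile class, printing a warning if it is not a Projectile.
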(event EventBeginPlay
  (bind _returnvalue (Actor|GetActorOfClass "/Game/Space/Player/BP_PlayerShip.BP_PlayerShip_C"))
  (Variables|Default|SetTargetActor _returnvalue))

(event EventTick
  (params (DeltaSeconds :type Float%20%28single-precision%29))
  (bind _targetactor (Variables|Default|GetTargetActor))
  (Class|LookatComponent|UpdateLookPosition (Variables|Default|GetLookAt) (.location (Transformation|GetActorTransform _targetactor)) (Transformation|GetVelocity _targetactor) (.MaxSpeed (Utilities|GetClassDefaults (Variables|Default|GetProjectileToPool))))
  (Class|GunComponent|Fire (Variables|Default|GetGun)))

(fn ConstructionScript
  (Variables|/Script/Space.GunComponent|SetProjectilePool (Variables|Default|GetGun) (Variables|Default|GetBulletPool))
  (bind _returnvalue (Class|PoolManagerComponent|GetClasstoPool (Variables|Default|GetBulletPool)))
  (bind _asprojectile (Utilities|Casting|CastToProjectileClass _returnvalue)
    (:then
      (Variables|Default|SetProjectileToPool _asprojectile))
    (:CastFailed
      (Variables|Default|SetProjectileToPool _asprojectile)
      (Development|PrintString "Projectile pool is not a projectile"))))