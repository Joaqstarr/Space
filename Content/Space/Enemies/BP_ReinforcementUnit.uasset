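; Reinforcement unit for space enemies that flies to a target and hands itself over as a transfer.
; A target change points the homing projectile movement at the root component of the target's owner.
; Each tick within a short fixed range of that owner, it calls OnReceiveTransfer on the target, repeating while in range.
; The unit destroys itself when OnTransferComplete fires.
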(event EventOnTargetChange
  (params (NewTarget :type Token%20Consumer%20Object%20Reference))
  (bind _output_get (Variables|Default|SetTarget NewTarget))
  (if (Utilities|IsValid _output_get)
    (Variables|/Script/Engine.ProjectileMovementComponent|SetHomingTargetComponent (Variables|Default|GetProjectileMovement) (Variables|/Script/Engine.Actor|GetRootComponent (Components|GetOwner _output_get)))))

(event EventOnTransferComplete
  (Actor|DestroyActor))

(event EventTick
  (params (DeltaSeconds :type Float%20%28single-precision%29))
  (if (Utilities|IsValid (Variables|Default|GetTarget))
    (if (< (Math|Vector|Distance(Vector) (Transformation|GetActorLocation) (Transformation|GetActorLocation (Components|GetOwner (Variables|Default|GetTarget)))) 2e+02)
      (Class|TokenConsumer|OnReceiveTransfer (Variables|Default|GetTarget) self))))

(fn ConstructionScript)