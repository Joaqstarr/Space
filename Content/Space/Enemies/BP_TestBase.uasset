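; Test enemy base that trades tokens with other token consumers by sending and receiving physical reinforcement units.
; Its TokenConsumer handles token requests and binds a transfer-sent event; SendReinforcements spawns a homing BP_ReinforcementUnit carrying the amount toward the target's owner.
; Overlapping units the base does not own deposit their tokens and are destroyed.
; A debug text widget shows the current token count every tick.
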(event Custom|Destroy%20Base
  (Class|TokenConsumer|UnregisterConsumer (Variables|Default|GetTokenConsumer)))

(event Custom|Request%20Reinforcements
  (Class|TokenConsumer|RequestTokens (Variables|Default|GetTokenConsumer) (Variables|Default|GetReinforcements%20Requested)))

(event Collision|EventActorBeginOverlap
  (params (OtherActor :type Actor%20Object%20Reference))
  (if (not (== (Components|GetOwner OtherActor) self))
    (bind _asbp_reinforcement_unit (Utilities|Casting|CastToBP_ReinforcementUnit OtherActor))
    (Class|TokenConsumer|OnReceiveTransfer (Variables|Default|GetTokenConsumer) (Variables|/Game/Space/Enemies/BP_ReinforcementUnit.BP_ReinforcementUnit_C|GetTokens%20Held _asbp_reinforcement_unit))
    (Actor|DestroyActor _asbp_reinforcement_unit)))

(event EventTick
  (params (DeltaSeconds :type Float%20%28single-precision%29))
  (Default|UpdateText (Variables|Default|GetText) (Utilities|Text|ToText(Integer) (Class|TokenConsumer|GetTokens (Variables|Default|GetTokenConsumer)))))

(event EventBeginPlay
  (bind _aswb_debug_text (Utilities|Casting|CastToWB_DebugText (UserInterface|GetWidget (Variables|Default|GetTextWidgetComponent))))
  (Variables|Default|SetText _aswb_debug_text)
  (EventDispatchers|BindEventtoOnTransferSent (Variables|Default|GetTokenConsumer) (EventDispatchers|CreateEvent :!event SendReinforcements))
  (Utilities|String|LogString "BASE CONSTRUCTED!"))

(fn ConstructionScript)

(fn SendReinforcements
  (params (Target :type Token%20Consumer%20Object%20Reference) (Amount :type Integer))
  (Development|PrintString (Utilities|String|Append "Sending " (Utilities|String|ToString(Integer) Amount) " tokens to " (Utilities|GetDisplayName Target)))
  (bind _returnvalue (Game|SpawnActorfromClass "/Game/Space/Enemies/BP_ReinforcementUnit.BP_ReinforcementUnit_C" (Transformation|GetActorTransform) "Undefined" "MultiplyWithRoot" self 0))
  (bind _output_get (LocalVariables|SetPayload _returnvalue))
  (Variables|/Game/Space/Enemies/BP_ReinforcementUnit.BP_ReinforcementUnit_C|SetTokens%20Held _output_get Amount)
  (Variables|/Script/Engine.ProjectileMovementComponent|SetHomingTargetComponent (Variables|/Game/Space/Enemies/BP_ReinforcementUnit.BP_ReinforcementUnit_C|GetProjectileMovement (LocalVariables|GetPayload)) (Variables|/Script/Engine.Actor|GetRootComponent (Components|GetOwner Target))))