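; BP_EnemyShip is an enemy ship that chases the player ship in the space game.
; It caches the BP_PlayerShip on BeginPlay and feeds its location to the ChaseAi component every Tick, alongside a debug print of the child actor count.
; When HealthComponent reports depleted health, it destroys all child actors, then itself.
; DirToPlayer returns a normalized vector that, despite its name, points from player to enemy.
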(event OnHealthDepleted(HealthComponent)
  (for _array_element (Actor|GetAllChildActors true)
    (Actor|DestroyActor _array_element))
  (Actor|DestroyActor))

(event EventBeginPlay
  (bind _returnvalue (Actor|GetActorOfClass "/Game/Space/Player/BP_PlayerShip.BP_PlayerShip_C"))
  (Variables|Default|SetPlayer _returnvalue))

(event Collision|EventActorBeginOverlap
  (params (OtherActor :type Actor%20Object%20Reference)))

(event EventTick
  (params (DeltaSeconds :type Float%20%28single-precision%29))
  (Class|ChaseAiComponent|UpdateTargetPosition (Variables|Default|GetChaseAi) (Transformation|GetActorLocation (Variables|Default|GetPlayer)))
  (Development|PrintString (Utilities|String|ToString(Integer) (Utilities|Array|Length (Actor|GetAllChildActors true))) true true "(R=0.000000,G=0.660000,B=1.000000,A=1.000000)" 2.0 "76"))

(fn ConstructionScript)

(fn DirtoPlayer
  (return (Math|Vector|Normalize (- (Transformation|GetActorLocation) (Transformation|GetActorLocation (Variables|Default|GetPlayer))))))