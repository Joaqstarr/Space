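; BP_EnemyShip is an enemy ship that chases the player ship in the space game.
; On BeginPlay it caches the BP_PlayerShip, then feeds that ship's location to its ChaseAi component every tick.
; When its HealthComponent reports depleted health, it destroys all child actors and then itself.
; The DirToPlayer helper, uncalled here, returns a normalized vector that points from the player toward the enemy, despite its name.
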(event OnHealthDepleted(HealthComponent)
  (for _array_element (Actor|GetAllChildActors true)
    (Actor|DestroyActor _array_element))
  (Actor|DestroyActor))

(event EventBeginPlay
  (bind _returnvalue (Actor|GetActorOfClass "/Game/Space/Player/BP_PlayerShip.BP_PlayerShip_C"))
  (Variables|Default|SetPlayer _returnvalue))

(event Collision|EventActorBeginOverlap
  (params (OtherActor :type Actor%20Object%20Reference)))

(event EventTick
  (params (DeltaSeconds :type Float%20%28single-precision%29))
  (Class|ChaseAiComponent|UpdateTargetPosition (Variables|Default|GetChaseAi) (Transformation|GetActorLocation (Variables|Default|GetPlayer))))

(fn ConstructionScript)

(fn DirtoPlayer
  (return (Math|Vector|Normalize (- (Transformation|GetActorLocation) (Transformation|GetActorLocation (Variables|Default|GetPlayer))))))