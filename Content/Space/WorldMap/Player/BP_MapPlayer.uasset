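; BP_MapPlayer is the player-controlled pawn for the space world map.
; Client-side possess and unpossess events add and remove the IMC_Map Enhanced Input mapping context on the player controller's local player subsystem.
; The IA_Move action value is passed as a world-space direction to TryAddMovementInput, scaled by MoveSpeed.
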(event Input|EnhancedActionEvents|EnhancedInputActionIA_Move
  (params (ActionValue :type Vector :default "0, 0, 0") (ElapsedSeconds :type Float%20%28double-precision%29) (TriggeredSeconds :type Float%20%28double-precision%29) (InputAction :type Input%20Action%20Object%20Reference :default "/Game/Space/Input/IA_Move.IA_Move"))
  (Class|MapPlayer|TryAddMovementInput ActionValue (Variables|Default|GetMoveSpeed)))

(event EventBeginPlay)

(event Collision|EventActorBeginOverlap
  (params (OtherActor :type Actor%20Object%20Reference)))

(event EventTick
  (params (DeltaSeconds :type Float%20%28single-precision%29)))

(event EventUnPosessedClientBP
  (params (OldController :type Controller%20Object%20Reference))
  (bind _asplayer_controller (Utilities|Casting|CastToPlayerController OldController))
  (Utilities|IsValid _asplayer_controller
    (:Is%20Valid
      (Input|RemoveMappingContext (PlayerController|LocalPlayerSubsystems|GetEnhancedInputLocalPlayerSubsystem _asplayer_controller) "/Game/Space/Input/Map/IMC_Map.IMC_Map" (Utilities|Struct|MakeModifyContextOptions true false false)))))

(event EventPosessedClientBP
  (params (NewController :type Controller%20Object%20Reference))
  (bind _asplayer_controller (Utilities|Casting|CastToPlayerController NewController))
  (Utilities|IsValid _asplayer_controller
    (:Is%20Valid
      (Input|AddMappingContext (PlayerController|LocalPlayerSubsystems|GetEnhancedInputLocalPlayerSubsystem _asplayer_controller) "/Game/Space/Input/Map/IMC_Map.IMC_Map" 0 "(bIgnoreAllPressedKeysUntilRelease=True,bForceImmediately=False,bNotifyUserSettings=False)"))))

(fn ConstructionScript)