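; BP_testSword is a test sword Blueprint that fades its SMWingBlade mesh in and out through the "AmtVisible" material scalar.
; TurnOnSword plays a timeline whose SwordActivation track drives that parameter between 0 and 1, and TurnOffSword reverses it.
; ToggleSword picks either event from the SwordOn flag without changing the flag.
; The construction script sets the blade fully visible or hidden from the same flag.
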(event Custom|TurnOnSword
  (bind _swordactivation (Timeline|Timeline Play)
    (:Update
      (Rendering|Material|SetScalarParameterValueonMaterials (Variables|Default|GetSM_WingBlade) "AmtVisible" (Math|Float|Lerp 0.0 1.0 _swordactivation)))))

(event Custom|TurnOffSword
  (bind _swordactivation (Timeline|Timeline Reverse)
    (:Update
      (Rendering|Material|SetScalarParameterValueonMaterials (Variables|Default|GetSM_WingBlade) "AmtVisible" (Math|Float|Lerp 0.0 1.0 _swordactivation)))))

(event Custom|ToggleSword
  (if (Variables|Default|GetSwordOn)
    (CallFunction|TurnonSword)
    (else
      (CallFunction|TurnOffSword))))

(event EventBeginPlay)

(event Collision|EventActorBeginOverlap
  (params (OtherActor :type Actor%20Object%20Reference)))

(event EventTick
  (params (DeltaSeconds :type Float%20%28single-precision%29)))

(fn ConstructionScript
  (if (Variables|Default|GetSwordOn)
    (Rendering|Material|SetScalarParameterValueonMaterials (Variables|Default|GetSM_WingBlade) "AmtVisible" 1.0)
    (else
      (Rendering|Material|SetScalarParameterValueonMaterials (Variables|Default|GetSM_WingBlade) "AmtVisible" 0.0))))